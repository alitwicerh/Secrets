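; Door actor that swings open or closed on its yaw axis and shows an interaction icon by proximity.
; Entering or leaving the BoxColl volume toggles the Icon's visibility.
; The OpenDoor event plays or reverses a timeline based on its current track value, and the timeline's update sets the Door's relative rotation.
; The player input enable and disable nodes are disconnected, so OpenDoor relies on an external caller.
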(event OnComponentBeginOverlap(BoxColl)
  (params (OverlappedComponent :type Primitive%20Component%20Object%20Reference) (OtherActor :type Actor%20Object%20Reference) (OtherComp :type Primitive%20Component%20Object%20Reference) (OtherBodyIndex :type Integer) (bFromSweep :type Boolean) (SweepResult :type Hit%20Result%20Structure%20%28by%20ref%29))
  (Rendering|ToggleVisibility (Variables|Default|Geticon) false))

(event OnComponentEndOverlap(BoxColl)
  (params (OverlappedComponent :type Primitive%20Component%20Object%20Reference) (OtherActor :type Actor%20Object%20Reference) (OtherComp :type Primitive%20Component%20Object%20Reference) (OtherBodyIndex :type Integer))
  (Rendering|ToggleVisibility (Variables|Default|Geticon) false))

(event EventBeginPlay)

(event EventOpenDoor
  (if (< -1.0 (stale _newtrack_0))
    (bind _newtrack_0 (Timeline|Timeline_0 Play)
      (:Update
        (Transformation|SetRelativeRotation (Variables|Default|GetDoor) (Math|Rotator|MakeRotator 0.0 0.0 _newtrack_0) false false)))
    (else
      (Timeline|Timeline_0 Reverse))))

(fn ConstructionScript)