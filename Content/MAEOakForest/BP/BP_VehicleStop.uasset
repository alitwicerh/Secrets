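; Trigger volume that ends the truck ride and hands control back to the first-person character.
; When the truck enters the box, it stops with brake sound and timed throttle and brake inputs, and the listed car rails are destroyed.
; After a delay, it teleports the character to a drop-off point, possesses it, shows a mission hint to find the corpse, then destroys itself.
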(event OnComponentBeginOverlap(Box)
  (params (OverlappedComponent :type Primitive%20Component%20Object%20Reference) (OtherActor :type Actor%20Object%20Reference) (OtherComp :type Primitive%20Component%20Object%20Reference) (OtherBodyIndex :type Integer) (bFromSweep :type Boolean) (SweepResult :type Hit%20Result%20Structure%20%28by%20ref%29))
  (bind _returnvalue (Game|GetPlayerController 0))
  (bind _playerdown (Variables|Default|GetPlayerDown))
  (bind (_location _rotation) (Math|Transform|BreakTransform _playerdown))
  (bind _asbp_vehicle_04_truck (Utilities|Casting|CastToBP_vehicle04_Truck OtherActor))
  (Default|VehicleStop _asbp_vehicle_04_truck)
  (Default|StartBrakeSound _asbp_vehicle_04_truck)
  (Class|ChaosVehicleMovementComponent|SetThrottleInput (Variables|/Script/ChaosVehicles.WheeledVehiclePawn|GetVehicleMovementComponent _asbp_vehicle_04_truck) 0.6)
  (Utilities|FlowControl|Delay 0.2)
  (Class|ChaosVehicleMovementComponent|SetBrakeInput (Variables|/Script/ChaosVehicles.WheeledVehiclePawn|GetVehicleMovementComponent _asbp_vehicle_04_truck) 1.0)
  (for _array_element (Variables|Default|GetCarRails)
    (Actor|DestroyActor _array_element))
  (Utilities|FlowControl|Delay 1.0)
  (Class|ChaosVehicleMovementComponent|SetThrottleInput (Variables|/Script/ChaosVehicles.WheeledVehiclePawn|GetVehicleMovementComponent _asbp_vehicle_04_truck) 0.0)
  (Class|ChaosVehicleMovementComponent|SetBrakeInput (Variables|/Script/ChaosVehicles.WheeledVehiclePawn|GetVehicleMovementComponent _asbp_vehicle_04_truck) 0.0)
  (Utilities|FlowControl|Delay 5.5)
  (bind _returnvalue_2 (Actor|GetActorOfClass "/Game/FirstPerson/Blueprints/BP_FirstPersonCharacter.BP_FirstPersonCharacter_C"))
  (Transformation|Teleport _returnvalue_2 (+ (Transformation|GetActorLocation) _location) _rotation)
  (Pawn|Possess _returnvalue _returnvalue_2)
  (Input|SetInputModeGameOnly _returnvalue true)
  (bind _returnvalue_3 (UserInterface|CreateWidget "/Game/MAEOakForest/BP/w_Mision.w_Mision_C" _returnvalue "Find the corpse in the house"))
  (UserInterface|Viewport|AddtoViewport _returnvalue_3 0)
  (Default|GetHint _returnvalue_3 "Find the corpse in the house")
  (Actor|DestroyActor))

(fn ConstructionScript)