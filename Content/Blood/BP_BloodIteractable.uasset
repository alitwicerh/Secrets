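; BP_BloodIteractable is a blood decal that gets erased while a component tagged "Mopa" (mop) overlaps its box.
; The construction script creates a dynamic decal material and caches its base DistortionAmount.
; Overlap plays the Ereasing timeline, which scales that distortion by its alpha curve and destroys the actor when finished.
; Ending the overlap stops the timeline, so the next one resumes from that point.
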(event OnComponentBeginOverlap(Box)
  (params (OverlappedComponent :type Primitive%20Component%20Object%20Reference) (OtherActor :type Actor%20Object%20Reference) (OtherComp :type Primitive%20Component%20Object%20Reference) (OtherBodyIndex :type Integer) (bFromSweep :type Boolean) (SweepResult :type Hit%20Result%20Structure%20%28by%20ref%29))
  (if (Components|ComponentHasTag OtherComp "Mopa")
    (bind _dissapearingalpha (Timeline|Ereasing Play)
      (:Update
        (Audio|Parameter|SetFloatParameter (Variables|Default|GetBloodDecalMaterialInstance) "DistortionAmount" (* _dissapearingalpha (Variables|Default|GetBaseDistorionValue)) :!class /Script/AudioExtensions.AudioParameterControllerInterface))
      (:Finished
        (Actor|DestroyActor)))))

(event OnComponentEndOverlap(Box)
  (params (OverlappedComponent :type Primitive%20Component%20Object%20Reference) (OtherActor :type Actor%20Object%20Reference) (OtherComp :type Primitive%20Component%20Object%20Reference) (OtherBodyIndex :type Integer))
  (if (Components|ComponentHasTag OtherComp "Mopa")
    (bind _dissapearingalpha (Timeline|Ereasing Stop)
      (:Update
        (Audio|Parameter|SetFloatParameter (Variables|Default|GetBloodDecalMaterialInstance) "DistortionAmount" (* _dissapearingalpha (Variables|Default|GetBaseDistorionValue)) :!class /Script/AudioExtensions.AudioParameterControllerInterface))
      (:Finished
        (Actor|DestroyActor)))))

(fn ConstructionScript
  (bind _returnvalue (Rendering|Material|CreateDynamicMaterialInstance (Variables|Default|GetMaterial) "None" "None" :!class /Script/Engine.KismetMaterialLibrary))
  (Rendering|Components|Decal|SetDecalMaterial (Variables|Default|GetDecal) _returnvalue)
  (bind _output_get (Variables|Default|SetBloodDecalMaterialInstance _returnvalue))
  (bind _returnvalue_2 (Rendering|Material|GetScalarParameterValue _output_get "DistortionAmount" :!class /Script/Engine.MaterialInstanceDynamic))
  (Variables|Default|SetBaseDistorionValue _returnvalue_2))